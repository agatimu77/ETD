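; BP_Interactable is an interactable object that changes its cube's colour while it has focus.
; On BeginPlay it creates a dynamic material instance from Mat_Pilar on the Cube and caches the "Param" vector as the default colour.
; StartFocus and EndFocus call their parent implementations, then set that parameter to the focused colour or restore the cached default.
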(event `self.ReceiveBeginPlay`
  ;[1 1 1] storing colour details
  (bind _returnvalue (`PrimitiveComponent.CreateDynamicMaterialInstance` (`self.Cube`) 0 "/Game/Assets/Materiales/Mat_Pilar.Mat_Pilar" "None"))
  (bind _output_get (set `self.material Instance` _returnvalue))
  (bind _returnvalue_2 (`MaterialInstanceDynamic.K2_GetVectorParameterValue` _output_get "Param"))
  (set `self.DefaultColour` _returnvalue_2))

(event `ETDInteractableInterface.StartFocus`
  (`parent.StartFocus`)
  (`MaterialInstanceDynamic.SetVectorParameterValue` (`self.material Instance`) "Param" (`self.FocusedColour`)))

(event `ETDInteractableInterface.EndFocus`
  (`parent.EndFocus`)
  (`MaterialInstanceDynamic.SetVectorParameterValue` (`self.material Instance`) "Param" (`self.DefaultColour`)))

(fn `UserConstructionScript`)