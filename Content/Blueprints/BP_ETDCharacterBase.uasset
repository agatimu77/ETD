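; Base player character Blueprint that sets up the on-screen UI and keeps the health display current.
; On BeginPlay it creates crosshair and HUD widgets, then seeds the HUD from the ETDHealth component, refreshing it on AnyDamage.
; TraceForward only calls the parent implementation.
; The interact-message and camera line-trace nodes are unconnected and never run.
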(event `self.TraceForward`
  (`parent.TraceForward`))

(event `self.ReceiveBeginPlay`
  (bind _etdhealth (`self.ETDHealth`))
  (bind _returnvalue (`|CreateWidget` "/Game/Blueprints/BP_WidgetCrosshear.BP_WidgetCrosshear_C"))
  (`UserWidget.AddToViewport` _returnvalue 0)
  (bind _returnvalue_2 (`|CreateWidget` "/Game/Blueprints/BP_WidgetHUD.BP_WidgetHUD_C"))
  (bind _output_get (set `self.HUD` _returnvalue_2))
  (`UserWidget.AddToViewport` _output_get 0)
  (`/Game/Blueprints/BP_WidgetHUD.UpdateHealth` (`self.HUD`) (`ETDHealth.Health` _etdhealth) (`ETDHealth.DefaultHealth` _etdhealth)))

(event `self.StaticMeshComp.OnComponentBeginOverlap`
  (params (OverlappedComponent :type "PrimitiveComponent Object Reference") (OtherActor :type "Actor Object Reference") (OtherComp :type "PrimitiveComponent Object Reference") (OtherBodyIndex :type Integer) (bFromSweep :type Boolean) (SweepResult :type "HitResult Structure (by ref)")))

(event `self.ReceiveAnyDamage`
  (params (Damage :type "Float (single-precision)") (DamageType :type "DamageType Object Reference") (InstigatedBy :type "Controller Object Reference") (DamageCauser :type "Actor Object Reference"))
  (bind _etdhealth (`self.ETDHealth`))
  (`/Engine/EditorBlueprintResources/StandardMacros.IsValid` (`self.HUD`)
    (:`Is Valid`
      (`/Game/Blueprints/BP_WidgetHUD.UpdateHealth` (`self.HUD`) (`ETDHealth.Health` _etdhealth) (`ETDHealth.DefaultHealth` _etdhealth)))))

(fn `UserConstructionScript`)